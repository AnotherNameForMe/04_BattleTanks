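; Player-controllable tank pawn Blueprint that wires its components together and routes input to them.
; On BeginPlay it hands the barrel and turret to the TankAim component and both tracks to the TankMovement component.
; Aim axes rotate an azimuth gimbal and elevation spring arm for frame-rate-independent camera orbit, while fire, move and turn inputs forward to those components.
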(event `self.ReceiveBeginPlay`
  (`TankAimComponent.Initialise` (`self.TankAim`) (`self.TankBarrel`) (`self.TankTurret`))
  (`TankMovementComponent.Initialise` (`self.TankMovement`) (`self.TankTrackLeft`) (`self.TankTrackRight`)))

(event `InputAxis|AimAzimuth`
  (params (AxisValue :type "Float (single-precision)"))
  ;[1 1 1] Camera Control
  (`SceneComponent.K2_AddLocalRotation` (`self.Azimuth_Gimbal`) (`KismetMathLibrary.MakeRotator` 0.0 0.0 (* AxisValue (`GameplayStatics.GetWorldDeltaSeconds`) 100.0)) false false))

(event `InputAxis|AimAltitude`
  (params (AxisValue :type "Float (single-precision)"))
  ;[1 1 1] Camera Control
  (`SceneComponent.K2_AddLocalRotation` (`self.Elevation_SpringArm`) (`KismetMathLibrary.MakeRotator` 0.0 (* AxisValue (`GameplayStatics.GetWorldDeltaSeconds`) 100.0)) false false))

(event `InputAction|Fire`
  (params (Key :type "Key Structure"))
  ;[1 1 1] Fire Tank
  (:`Pressed`
    (`TankAimComponent.Fire` (`self.TankAim`))))

(event `InputAxis|move`
  (params (AxisValue :type "Float (single-precision)"))
  ;[1 1 1] Move and Turn
  (`TankMovementComponent.IntendMoveForward` (`self.TankMovement`) AxisValue))

(event `InputAxis|Turn`
  (params (AxisValue :type "Float (single-precision)"))
  ;[1 1 1] Move and Turn
  (`TankMovementComponent.IntendRotate` (`self.TankMovement`) AxisValue))

(fn `UserConstructionScript`)